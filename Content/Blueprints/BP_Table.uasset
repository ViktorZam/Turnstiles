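; BP_Table is an interactable table that lets the player swap between taking cards from its Cards array.
; Interact checks whether the first card is hidden and calls TakeCard with the second card if so, otherwise with the first.
; TakeCard hides the chosen card, reveals all others, and prints a Russian on-screen message naming the taken card by its first actor tag.
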(event EventBeginPlay)

(event Collision|EventActorBeginOverlap
  (params (OtherActor :type Actor%20Object%20Reference)))

(event EventTick
  (params (DeltaSeconds :type Float%20%28single-precision%29)))

(event EventInteract
  (if (Variables|/Script/Engine.Actor|GetbHidden (Utilities|Array|Get(acopy) (Variables|Default|GetCards)))
    (CallFunction|TakeCard 1)
    (else
      (CallFunction|TakeCard))))

(fn ConstructionScript
  (|CallParentFunction))

(fn TakeCard
  (params (NumCardInArray :type Integer))
  (for (_ _array_index) (Variables|Default|GetCards)
    (if (!= _array_index NumCardInArray)
      (Rendering|SetActorHiddenInGame (Utilities|Array|Get(acopy) (Variables|Default|GetCards) _array_index) false)
      (else
        (Rendering|SetActorHiddenInGame (Utilities|Array|Get(acopy) (Variables|Default|GetCards) NumCardInArray) true))))
  (Development|PrintString (Utilities|String|Append "Вы взяли карточку №" (Utilities|String|ToString(Name) (Utilities|Array|Get(acopy) (Variables|/Script/Engine.Actor|GetTags (Utilities|Array|Get(acopy) (Variables|Default|GetCards) NumCardInArray))))) true true "(R=0.000000,G=1.000000,B=0.001143,A=1.000000)" 4.0))