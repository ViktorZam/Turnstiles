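; BP_TurnstileBase is an interactable turnstile that slides its Blockage open only when its Card is hidden.
; Interact starts a timeline moving the Blockage along relative X, ignoring repeat presses while it moves or waits, and otherwise shows a different Indicator material.
; A two-second timer resets the Indicator and reverses the timeline if fully open.
; The construction script caches the start position and derives slide direction from the Card's first tag.
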(event Custom|StartDelay
  (bind _returnvalue (Utilities|Time|SetTimerbyEvent (delegate Custom|ReturnIndicator) 2.0))
  (Variables|Default|SetTimerReturnBlockage _returnvalue))

(event Custom|ReturnIndicator
  (Rendering|Material|SetMaterial (Variables|Default|GetIndicator) 0 "/Engine/BasicShapes/BasicShapeMaterial.BasicShapeMaterial")
  (if (Math|Float|NearlyEqual(Float) (.x (Variables|/Script/Engine.SceneComponent|GetRelativeLocation (Variables|Default|Getblockage))) (+ (.x (Variables|Default|GetStartRelativeLocationBlockage)) (* (Variables|Default|GetMultiplyForSide) 3.2e+02)) 5.0)
    (CallFunction|ReturnBlockage)))

(event Custom|ReturnBlockage
  (bind _blockage (Variables|Default|Getblockage))
  (bind _relativelocation (Variables|/Script/Engine.SceneComponent|GetRelativeLocation _blockage))
  (bind _alpha (Timeline|Timeline_MovingBlockage Reverse)
    (:Update
      (Transformation|SetRelativeLocation (Variables|Default|Getblockage) (Math|Vector|MakeVector (Math|Float|Lerp (.x (Variables|Default|GetStartRelativeLocationBlockage)) (+ (.x (Variables|Default|GetStartRelativeLocationBlockage)) (* (Variables|Default|GetMultiplyForSide) 3.2e+02)) _alpha) (.y _relativelocation) (.z _relativelocation)) false false))
    (:Finished
      (if (not (Math|Float|NearlyEqual(Float) (.x (Variables|Default|GetStartRelativeLocationBlockage)) (.x (Variables|/Script/Engine.SceneComponent|GetRelativeLocation (Variables|Default|Getblockage))) 5.0))
        (CallFunction|StartDelay)))))

(event EventInteract
  (bind _blockage (Variables|Default|Getblockage))
  (bind _relativelocation (Variables|/Script/Engine.SceneComponent|GetRelativeLocation _blockage))
  (if (Variables|/Script/Engine.Actor|GetbHidden (Variables|Default|GetCard))
    ;[1 1 1] Проверки для того чтобы при многократном нажатии створка многократно не отводилась
    (if (not (Components|Activation|IsActive (Variables|Default|GetTimeline_MovingBlockage)))
      (if (not (Utilities|Time|IsTimerActivebyHandle (Variables|Default|GetTimerReturnBlockage)))
        (Rendering|Material|SetMaterial (Variables|Default|GetIndicator) 0 "/Engine/MapTemplates/Materials/BasicAsset03.BasicAsset03")
        (bind _alpha (Timeline|Timeline_MovingBlockage Play)
          (:Update
            (Transformation|SetRelativeLocation (Variables|Default|Getblockage) (Math|Vector|MakeVector (Math|Float|Lerp (.x (Variables|Default|GetStartRelativeLocationBlockage)) (+ (.x (Variables|Default|GetStartRelativeLocationBlockage)) (* (Variables|Default|GetMultiplyForSide) 3.2e+02)) _alpha) (.y _relativelocation) (.z _relativelocation)) false false))
          (:Finished
            (if (not (Math|Float|NearlyEqual(Float) (.x (Variables|Default|GetStartRelativeLocationBlockage)) (.x (Variables|/Script/Engine.SceneComponent|GetRelativeLocation (Variables|Default|Getblockage))) 5.0))
              (CallFunction|StartDelay))))))
    (else
      (Rendering|Material|SetMaterial (Variables|Default|GetIndicator) 0 "/Engine/MapTemplates/Materials/BasicAsset01.BasicAsset01")
      (CallFunction|StartDelay))))

(fn ConstructionScript
  (Variables|Default|SetStartRelativeLocationBlockage (Variables|/Script/Engine.SceneComponent|GetRelativeLocation (Variables|Default|Getblockage)))
  (switch name (Utilities|Array|Get(acopy) (Variables|/Script/Engine.Actor|GetTags (Variables|Default|GetCard)))
    (:1
      (Variables|Default|SetMultiplyForSide -1.0))
    (:2
      (Variables|Default|SetMultiplyForSide 1.0))))